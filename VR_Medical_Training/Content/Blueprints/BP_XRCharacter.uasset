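; BP_XRCharacter is the player character for XR, setting up head-mounted display tracking and hand controllers when play begins.
; With an HMD enabled, SetupVR uses a local-floor tracking origin and adds the default and hands Enhanced Input mapping contexts.
; SetupHands spawns separate left and right hand controller actors owned by the character and attaches them to its Origin component.
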(event EventBeginPlay
  (Utilities|FlowControl|Sequence
    (:then_0
      (|SetupVR))
    (:then_1
      (|SetupHands))))

(fn ConstructionScript)
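; BP_Cart is a cart Blueprint whose drawers are GrabbableDrawer child actors.
; On BeginPlay it scans its ChildActorComponents and passes each drawer its component's world location and a shared DrawerOffsetMax through SetMaxOffset.
; Tick and the construction script are empty.
; Leftover disconnected nodes show abandoned attempts to move a drawer component directly from the cart, with notes on moving clamping into a handle actor.
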(event EventTick
  (params (DeltaSeconds :type Float%20%28single-precision%29)))

(event EventBeginPlay
  (for _array_element (Actor|GetComponentsByClass "/Script/Engine.ChildActorComponent")
    (bind _asgrabbable_drawer (Utilities|Casting|CastToGrabbableDrawer (Variables|/Script/Engine.ChildActorComponent|GetChildActor _array_element)))
    (Class|GrabbableDrawer|SetMaxOffset _asgrabbable_drawer (Transformation|GetWorldLocation _array_element) (Variables|Default|GetDrawerOffsetMax))))

(fn ConstructionScript)
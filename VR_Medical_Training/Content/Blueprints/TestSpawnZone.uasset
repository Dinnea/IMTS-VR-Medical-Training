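; TestSpawnZone is an actor that spawns a scalpel at its own transform on BeginPlay and flags it when it enters the zone.
; It sets itself as the scalpel's SpawnZone and keeps a reference to it as Spawned.
; When that spawned actor begins overlapping, it casts it to GrababbleItem and sets OnSpawn to true; end overlap does nothing.
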(event EventBeginPlay
  (bind _returnvalue (Game|SpawnActorfromClass "/Game/Blueprints/BP_Scalpel.BP_Scalpel_C" (Transformation|GetActorTransform) "Undefined" "MultiplyWithRoot" 0 0))
  (Variables|/Script/VR_Medical_Training.GrababbleItem|SetSpawnZone _returnvalue self)
  (Variables|Default|SetSpawned _returnvalue))

(event Collision|EventActorBeginOverlap
  (params (OtherActor :type Actor%20Object%20Reference))
  (bind _spawned (Variables|Default|GetSpawned))
  (if (== OtherActor _spawned)
    (bind _asgrababble_item (Utilities|Casting|CastToGrababbleItem _spawned))
    (Variables|/Script/VR_Medical_Training.GrababbleItem|SetOnSpawn _asgrababble_item true)))

(event EventTick
  (params (DeltaSeconds :type Float%20%28single-precision%29)))

(event Collision|EventActorEndOverlap
  (params (OtherActor :type Actor%20Object%20Reference)))

(fn ConstructionScript)
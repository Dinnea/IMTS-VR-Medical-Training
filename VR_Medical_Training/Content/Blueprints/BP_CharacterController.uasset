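; BP_CharacterController is a VR player setup Blueprint that initializes tracking, input and hand actors on BeginPlay.
; If a head-mounted display is enabled, it sets the tracking origin to local floor and adds the default and hands Enhanced Input mapping contexts at equal priority.
; It then spawns BP_LeftHand and BP_RightHand with itself as owner, regardless of the headset check.
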(event EventBeginPlay
  (bind _self self)
  (Utilities|FlowControl|Sequence
    (:then_0
      (if (Class|HeadMountedDisplayFunctionLibrary|IsHeadMountedDisplayEnabled)
        (Class|HeadMountedDisplayFunctionLibrary|SetTrackingOrigin "LocalFloor")
        (Input|AddMappingContext (PlayerController|LocalPlayerSubsystems|GetEnhancedInputLocalPlayerSubsystem (Game|GetPlayerController 0)) "/Game/XRFramework/Input/IMC_Default.IMC_Default" 0 "(bIgnoreAllPressedKeysUntilRelease=True,bForceImmediately=False,bNotifyUserSettings=False)")
        (Input|AddMappingContext "/Game/XRFramework/Input/IMC_Hands.IMC_Hands" 0 "(bIgnoreAllPressedKeysUntilRelease=True,bForceImmediately=False,bNotifyUserSettings=False)")))
    (:then_1
      (Utilities|FlowControl|Sequence
        (:then_0
          (Game|SpawnActorfromClass :Class "/Game/Blueprints/BP_LeftHand.BP_LeftHand_C" :CollisionHandlingOverride "Undefined" :TransformScaleMethod "MultiplyWithRoot" :Owner _self :Instigator 0))
        (:then_1
          (Game|SpawnActorfromClass :Class "/Game/Blueprints/BP_RightHand.BP_RightHand_C" :CollisionHandlingOverride "Undefined" :TransformScaleMethod "MultiplyWithRoot" :Owner _self :Instigator 0))))))

(fn ConstructionScript)